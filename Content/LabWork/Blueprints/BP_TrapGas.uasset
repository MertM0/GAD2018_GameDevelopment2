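; BP_TrapGas is a gas trap that drains the player's health while they stand inside its box.
; BeginPlay caches the Boris character and starts a looping one-second timer that deals damage only while the overlap flag is set.
; Box overlaps toggle that flag and pause or resume the timer.
; The player's OnTrapDeactivated event, for the matching trap type, disables box collision and deactivates the smoke Niagara effect.
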(event `self.Box.OnComponentBeginOverlap`
  (params (OverlappedComponent :type "PrimitiveComponent Object Reference") (OtherActor :type "Actor Object Reference") (OtherComp :type "PrimitiveComponent Object Reference") (OtherBodyIndex :type Integer) (bFromSweep :type Boolean) (SweepResult :type "HitResult Structure (by ref)"))
  ;[0.15 0.1337 0.001267 0.5] Collision Check
  (if (== OtherActor (`self.Player`))
    (set `self.CanDamage` true)
    (`KismetSystemLibrary.K2_UnPauseTimerHandle` (`self.Handle`))))

(event `self.Box.OnComponentEndOverlap`
  (params (OverlappedComponent :type "PrimitiveComponent Object Reference") (OtherActor :type "Actor Object Reference") (OtherComp :type "PrimitiveComponent Object Reference") (OtherBodyIndex :type Integer))
  ;[0.15 0.1337 0.001267 0.5] Collision Check
  (if (== OtherActor (`self.Player`))
    (set `self.CanDamage` false)
    (`KismetSystemLibrary.K2_PauseTimerHandle` (`self.Handle`))))

(event `self.ReceiveBeginPlay`
  (bind _asbp_boris_character (cast `/Game/LabWork/Blueprints/BP_BorisCharacter` (`GameplayStatics.GetPlayerCharacter` 0)))
  (bind _output_get (set `self.Player` _asbp_boris_character))
  (add `/Game/LabWork/Blueprints/BP_BorisCharacter.OnTrapDeactivated` _output_get (delegate `OnTrapDeactivated_Event`))
  (bind _returnvalue (`KismetSystemLibrary.K2_SetTimerDelegate` (delegate `GiveDamage`) 1.0 true))
  (set `self.Handle` _returnvalue))

(event `GiveDamage`
  ;[1 0 0 0.5] Damage
  (if (`self.CanDamage`)
    (`/Game/LabWork/Blueprints/BP_BorisCharacter.UpdateHealth` (`self.Player`) -5.0)))

(event `OnTrapDeactivated_Event`
  (params (TrapType :type "/Game/LabWork/Blueprints/Resources/E_TrapType Enum" :default "NewEnumerator0"))
  ; Deactivate
  (if (`|EnumEquality` TrapType "NewEnumerator2")
    (`PrimitiveComponent.SetCollisionEnabled` (`self.Box`) "NoCollision")
    (`ActorComponent.Deactivate` (`self.PS_FX_smoke_dungeon_Niagara`))))

(fn `UserConstructionScript`)