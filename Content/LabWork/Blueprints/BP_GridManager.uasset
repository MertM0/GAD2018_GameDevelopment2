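; BP_GridManager is an actor that builds a Rows by Columns grid of BP_MazeCell actors.
; GenerateGrid first destroys every BP_MazeCell in the world, then spawns new cells in a nested loop, offset from the manager by CellSize scaled by 100.
; Each cell receives CellSize and is attached to the manager's root with KeepRelative rules.
; BeginPlay and the construction script are empty, so neither triggers generation.
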(event `self.ReceiveBeginPlay`)

(event `GenerateGrid`
  (bind _outactors (`GameplayStatics.GetAllActorsOfClass` "/Game/LabWork/Blueprints/BP_MazeCell.BP_MazeCell_C"))
  (for _array_element _outactors
    (`self.K2_DestroyActor` _array_element))
  (for _index (range (`self.Rows`))
    (for _index_2 (range (`self.Columns`))
      (bind _returnvalue (`|SpawnActorFromClass` "/Game/LabWork/Blueprints/BP_MazeCell.BP_MazeCell_C" (`KismetMathLibrary.MakeTransform` (+ (`self.K2_GetActorLocation`) (`KismetMathLibrary.MakeVector` (* (* _index (`self.CellSize`)) 100.0) (* (* _index_2 (`self.CellSize`)) 100.0)))) "Undefined" "MultiplyWithRoot" null (`self.CellSize`) null))
      (`self.K2_AttachToComponent` _returnvalue (`self.DefaultSceneRoot`) "None" "KeepRelative" "KeepRelative" "KeepRelative" true))))

(fn `UserConstructionScript`)