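; BP_Gold is an interactable gold pickup that adds a random amount of gold to BP_BorisCharacter.
; The construction script rolls ItemGold, shows it on a TextRender and selects one of three coin meshes by value tier.
; Interact credits the player, removes the box and text components, then animates the mesh scale with a timeline and destroys the actor.
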(event `/Game/LabWork/Blueprints/Resources/BPI_Interactable.Interact`
  (bind _asbp_boris_character (cast `/Game/LabWork/Blueprints/BP_BorisCharacter` (`GameplayStatics.GetPlayerCharacter` 0)))
  (`/Game/LabWork/Blueprints/BP_BorisCharacter.UpdateGold` _asbp_boris_character (`self.ItemGold`))
  (`ActorComponent.K2_DestroyComponent` (`self.Box`))
  (`ActorComponent.K2_DestroyComponent` (`self.TextRender`))
  (bind (_direction _newtrack_0) (`Timeline|Timeline`)
    (:`Update`
      (`SceneComponent.SetRelativeScale3D` (`self.StaticMesh`) (`KismetMathLibrary.MakeVector` _newtrack_0 _newtrack_0 _newtrack_0)))
    (:`Finished`
      (`self.K2_DestroyActor`))))

(fn `UserConstructionScript`
  (bind _output_get (set `self.ItemGold` (`KismetMathLibrary.RandomIntegerInRange` 1 20)))
  (`TextRenderComponent.K2_SetText` (`self.TextRender`) (`KismetTextLibrary.Conv_IntToText` _output_get))
  (if (<= (`self.ItemGold`) 5)
    (`StaticMeshComponent.SetStaticMesh` (`self.StaticMesh`) "/Game/Packets/Fantastic_Dungeon_Pack/meshes/props/small_deco/SM_PROP_coin_dungeon_01.SM_PROP_coin_dungeon_01")
    (elif (<= (`self.ItemGold`) 12)
      (`StaticMeshComponent.SetStaticMesh` (`self.StaticMesh`) "/Game/Packets/Fantastic_Dungeon_Pack/meshes/props/small_deco/SM_PROP_coin_dungeon_03.SM_PROP_coin_dungeon_03")
      (else
        (`StaticMeshComponent.SetStaticMesh` (`self.StaticMesh`) "/Game/Packets/Fantastic_Dungeon_Pack/meshes/props/small_deco/SM_PROP_coin_dungeon_02.SM_PROP_coin_dungeon_02")))))