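; BP_SpawnManager is a key-driven manager actor that spawns and damages enemies, enabling input from player controller 0 on BeginPlay.
; F picks a random enemy type, gets its difficulty from a map and stats from DT_EnemyStats via the enum name, and prints the stats.
; It then spawns a BP_EnemyBase with that data at a random XY position and tracks it in a list.
; X damages every valid tracked enemy.
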(event `self.ReceiveBeginPlay`
  (`self.EnableInput` (`GameplayStatics.GetPlayerController` 0)))

(event `Key|F`
  (params (Key :type "Key Structure"))
  (:`Pressed`
    (bind _output_get (set `self.SpawnedEnemy` (`|GetArrayItem` (`self.EEnemyTypes`) (`KismetMathLibrary.RandomIntegerInRange` 0 3))))
    (set `self.SpawnedDifficulty` (`BlueprintMapLibrary.Map_Find` (`self.EnemyDifficulties`) _output_get))
    (bind _returnvalue (`|GetEnumeratorNameAsString` _output_get))
    (bind _returnvalue_2 (`|GetDataTableRow` "/Game/LabWork2/SpawnManager/DT_EnemyStats.DT_EnemyStats" (`KismetStringLibrary.Conv_StringToName` _returnvalue))
      (:`then`
        (bind _output_get_2 (set `self.SpawnedEnemyStats` _returnvalue_2))
        (bind (_health _damage _speed) (break `/Game/LabWork2/SpawnManager/ST_EnemyStats` _output_get_2))
        (`KismetSystemLibrary.PrintString` (`KismetStringLibrary.Concat_StrStr` "Health:" (`KismetStringLibrary.Conv_DoubleToString` _health) " Damage:" (`KismetStringLibrary.Conv_DoubleToString` _damage) " Speed:" (`KismetStringLibrary.Conv_DoubleToString` _speed) _returnvalue))
        (bind _returnvalue_3 (`|SpawnActorFromClass` "/Game/LabWork2/SpawnManager/BP_EnemyBase.BP_EnemyBase_C" (`KismetMathLibrary.MakeTransform` (`KismetMathLibrary.MakeVector` (`KismetMathLibrary.RandomFloatInRange` 100.0 1000.0) (`KismetMathLibrary.RandomFloatInRange` 100.0 1000.0) 10.0)) "Undefined" "MultiplyWithRoot" null (`self.SpawnedEnemy`) (`self.SpawnedEnemyStats`) (`self.SpawnedDifficulty`) null))
        (`KismetArrayLibrary.Array_Add` (`self.SpawnedEnemyList`) _returnvalue_3)))))

(event `Key|X`
  (params (Key :type "Key Structure"))
  (:`Pressed`
    (for _array_element (`self.SpawnedEnemyList`)
      (`/Engine/EditorBlueprintResources/StandardMacros.IsValid` _array_element
        (:`Is Valid`
          (`/Game/LabWork2/SpawnManager/BP_EnemyBase.TakeDamage` _array_element 50.0))))))

(fn `UserConstructionScript`)