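; BP_Shape is an actor that becomes one of several random shapes, with a mesh, material and text label naming its type.
; The construction script picks a random EShapeType and uses its name to look up DT_ShapeInfo for the mesh and material.
; A Selection function highlights it through a dynamic material instance with a high Emission value, or restores the table's material when deselected.
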(fn `Selection`
  (params (bSelect :type Boolean))
  (if bSelect
    ; Emissive Material
    (bind _returnvalue (`KismetMaterialLibrary.CreateDynamicMaterialInstance` (`self.Material`)))
    (`MaterialInstanceDynamic.SetScalarParameterValue` _returnvalue "Emission" 100.0)
    (`PrimitiveComponent.SetMaterial` (`self.StaticMesh`) 0 _returnvalue)
    (else
      ; Normal Material
      (`PrimitiveComponent.SetMaterial` (`self.StaticMesh`) 0 (`.Material_13_310A7836414DA3AADEF45F8E91EA19F0` (break `/Game/LabWork2/ST_ShapeInfo` (`self.ShapeInfo`)))))))

(fn `UserConstructionScript`
  (bind _staticmesh (`self.StaticMesh`))
  (bind _output_get (set `self.ShapeType` (`|GetArrayItem` (`self.EShapeType`) (`KismetMathLibrary.RandomIntegerInRange` 0 2))))
  (bind _returnvalue (`KismetStringLibrary.Conv_StringToName` (`|GetEnumeratorNameAsString` _output_get)))
  (bind _returnvalue_2 (`|GetDataTableRow` "/Game/LabWork2/DT_ShapeInfo.DT_ShapeInfo" _returnvalue)
    (:`then`
      (set `self.ShapeInfo` _returnvalue_2)
      (bind (_mesh _material) (break `/Game/LabWork2/ST_ShapeInfo` _returnvalue_2))
      (`StaticMeshComponent.SetStaticMesh` _staticmesh _mesh)
      (`PrimitiveComponent.SetMaterial` _staticmesh 0 _material)
      (set `self.Material` _material)
      (`TextRenderComponent.K2_SetText` (`self.TextRender`) (`KismetTextLibrary.Conv_NameToText` _returnvalue)))))