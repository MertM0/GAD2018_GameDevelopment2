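; BP_TrapSpike is a floor spike trap that damages the player character (BP_BorisCharacter) on contact.
; Overlapping its Box trigger deals fixed damage through the player's UpdateHealth and plays a timeline that lerps the spike mesh up from below the floor.
; On BeginPlay it binds to the player's trap-deactivated dispatcher, disabling the trigger's collision when the matching trap type is broadcast.
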(event `self.ReceiveBeginPlay`
  (bind _asbp_boris_character (cast `/Game/LabWork/Blueprints/BP_BorisCharacter` (`GameplayStatics.GetPlayerCharacter` 0)))
  (bind _output_get (set `self.Player` _asbp_boris_character))
  (add `/Game/LabWork/Blueprints/BP_BorisCharacter.OnTrapDeactivated` _output_get (delegate `OnTrapDeactivated_Event`)))

(event `OnTrapDeactivated_Event`
  (params (TrapType :type "/Game/LabWork/Blueprints/Resources/E_TrapType Enum" :default "NewEnumerator0"))
  ; Deactivate
  (if (`|EnumEquality` TrapType "NewEnumerator1")
    (`PrimitiveComponent.SetCollisionEnabled` (`self.Box`) "NoCollision")))

(event `self.Box.OnComponentBeginOverlap`
  (params (OverlappedComponent :type "PrimitiveComponent Object Reference") (OtherActor :type "Actor Object Reference") (OtherComp :type "PrimitiveComponent Object Reference") (OtherBodyIndex :type Integer) (bFromSweep :type Boolean) (SweepResult :type "HitResult Structure (by ref)"))
  (bind _player (`self.Player`))
  ;[1 0 0 0.5] Collision Check, Animation and Damage
  (if (== OtherActor _player)
    (`/Game/LabWork/Blueprints/BP_BorisCharacter.UpdateHealth` _player -10.0)
    (bind (_direction _newtrack_0) (`Timeline|Timeline` :!via `PlayFromStart`)
      (:`Update`
        (`SceneComponent.K2_SetRelativeLocation` (`self.SM_PROP_trap_floor_spikes_dungeon_05`) (`KismetMathLibrary.VLerp` (0.0 0.0 -110.0) (0.0 0.0 0.0) _newtrack_0) false false)))))

(fn `UserConstructionScript`)