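; BP_Door is a key-locked sliding door that opens only when the player holds the key of the required color.
; On BeginPlay it sets the mesh material from RequiredKeyColor, with cases for Red and Green.
; Interact checks the BP_BorisCharacter KeyInventory for that color, then a FlipFlop alternately plays and reverses the Door_Slide timeline, which lerps the mesh sideways along local X.
; Without the key, it prints an on-screen warning.
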(event `self.ReceiveBeginPlay`
  ; Set Door Color
  (switch `/Game/LabWork/Blueprints/Resources/E_KeyColors` (`self.RequiredKeyColor`)
    (:`NewEnumerator0`
      (`PrimitiveComponent.SetMaterial` (`self.StaticMesh`) 0 "/Engine/VREditor/LaserPointer/LaserPointerMaterialInst.LaserPointerMaterialInst"))
    (:`NewEnumerator1`
      (`PrimitiveComponent.SetMaterial` (`self.StaticMesh`) 0 "/Engine/VREditor/LaserPointer/LaserPointerMaterial_Inst.LaserPointerMaterial_Inst"))))

(event `/Game/LabWork/Blueprints/Resources/BPI_Interactable.Interact`
  ; Interact
  (bind _asbp_boris_character (cast `/Game/LabWork/Blueprints/BP_BorisCharacter` (`GameplayStatics.GetPlayerCharacter` 0)))
  (if (`KismetArrayLibrary.Array_Contains` (`/Game/LabWork/Blueprints/BP_BorisCharacter.KeyInventory` _asbp_boris_character) (`self.RequiredKeyColor`))
    (`/Engine/EditorBlueprintResources/StandardMacros.FlipFlop`
      (:`A`
        (bind (_direction _slideamount) (`Timeline|Door_Slide` :!label _label)
          (:`Update`
            (`SceneComponent.K2_SetRelativeLocation` (`self.StaticMesh`) (`KismetMathLibrary.VLerp` (0.0 0.0 0.0) (500.0 0.0 0.0) _slideamount) false false))))
      (:`B`
        (goto _label :!via `Reverse`)))
    (else
      (`KismetSystemLibrary.PrintString` "You don't have correct key!"))))

(fn `UserConstructionScript`)