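; BP_TrapAxe is a swinging blade trap that damages the player BP_BorisCharacter on overlap with its Box collision.
; A looping timer replays a timeline that lerps the blade mesh's rotation from side to side.
; It binds to the player's OnTrapDeactivated event and, for its matching trap type, disables collision, clears the timer, stops the timeline and resets the blade upright.
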(event `self.Box.OnComponentBeginOverlap`
  (params (OverlappedComponent :type "PrimitiveComponent Object Reference") (OtherActor :type "Actor Object Reference") (OtherComp :type "PrimitiveComponent Object Reference") (OtherBodyIndex :type Integer) (bFromSweep :type Boolean) (SweepResult :type "HitResult Structure (by ref)"))
  (bind _player (`self.Player`))
  ;[0.15 0.1337 0.001267 0.5] Collision Check
  (if (== OtherActor _player)
    (`/Game/LabWork/Blueprints/BP_BorisCharacter.UpdateHealth` _player -10.0)))

(event `self.ReceiveBeginPlay`
  (bind _asbp_boris_character (cast `/Game/LabWork/Blueprints/BP_BorisCharacter` (`GameplayStatics.GetPlayerCharacter` 0)))
  (bind _output_get (set `self.Player` _asbp_boris_character))
  (add `/Game/LabWork/Blueprints/BP_BorisCharacter.OnTrapDeactivated` _output_get (delegate `OnTrapDeactivated_Event`))
  (bind _returnvalue (`KismetSystemLibrary.K2_SetTimerDelegate` (delegate `Swing`) 2.0 true))
  (set `self.Handle` _returnvalue))

(event `Swing`
  ;[1 0 0 0.5] Swing Animation
  (bind (_direction _newtrack_0) (`Timeline|Timeline_0` :!via `PlayFromStart` :!label _label)
    (:`Update`
      (`SceneComponent.K2_SetRelativeRotation` (`self.SM_PROP_trap_blade_dungeon_02`) (`KismetMathLibrary.RLerp` (struct :`Pitch` 60.0) (struct :`Pitch` -60.0) _newtrack_0) false false))))

(event `OnTrapDeactivated_Event`
  (params (TrapType :type "/Game/LabWork/Blueprints/Resources/E_TrapType Enum" :default "NewEnumerator0"))
  ; Deactivate
  (if (`|EnumEquality` TrapType "NewEnumerator3")
    (`PrimitiveComponent.SetCollisionEnabled` (`self.Box`) "NoCollision")
    (`KismetSystemLibrary.K2_ClearAndInvalidateTimerHandle` (`self.Handle`))
    (`SceneComponent.K2_SetRelativeRotation` :`self` (`self.SM_PROP_trap_blade_dungeon_02`))
    (goto _label :!via `Stop`)))

(fn `UserConstructionScript`)