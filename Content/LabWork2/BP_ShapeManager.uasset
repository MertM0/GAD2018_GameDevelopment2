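; BP_ShapeManager spawns a row of five BP_Shape actors along Y from its own location and lets the player select and move them.
; BeginPlay stores them in an array, selects the first and enables input on the manager.
; E and Q step the selection through the array without wrapping, calling Selection on each affected shape.
; Keys 1 and 2 nudge the selected shape along world Y or Z, with 3 toggling the axis.
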(event `self.ReceiveBeginPlay`
  (bind (_returnvalue_x _returnvalue_y _returnvalue_z) (`KismetMathLibrary.BreakVector` (`self.K2_GetActorLocation`)))
  ; Spawn
  (for _index (range 5)
    (bind _returnvalue (`|SpawnActorFromClass` "/Game/LabWork2/BP_Shape.BP_Shape_C" (`KismetMathLibrary.MakeTransform` (`KismetMathLibrary.MakeVector` _returnvalue_x (+ _returnvalue_y (* _index 150)) _returnvalue_z)) "Undefined" "MultiplyWithRoot" null null))
    (`KismetArrayLibrary.Array_Add` (`self.SpawnedShapes`) _returnvalue))
  (`/Game/LabWork2/BP_Shape.Selection` (`|GetArrayItem` (`self.SpawnedShapes`)) true)
  (set `self.CurrentIndex` 0)
  (`self.EnableInput` (`GameplayStatics.GetPlayerController` 0)))

(event `Key|E`
  (params (Key :type "Key Structure"))
  ; Update Selection
  (:`Pressed`
    (if (< (`self.CurrentIndex`) (`KismetArrayLibrary.Array_LastIndex` (`self.SpawnedShapes`)))
      (`/Game/LabWork2/BP_Shape.Selection` (`|GetArrayItem` (`self.SpawnedShapes`) (`self.CurrentIndex`)) false)
      (bind _result (`/Engine/EditorBlueprintResources/StandardMacros.IncrementInt` (`self.CurrentIndex`))
        (:`  `
          (`/Game/LabWork2/BP_Shape.Selection` (`|GetArrayItem` (`self.SpawnedShapes`) _result) true))))))

(event `Key|Q`
  (params (Key :type "Key Structure"))
  ; Update Selection
  (:`Pressed`
    (if (> (`self.CurrentIndex`) 0)
      (`/Game/LabWork2/BP_Shape.Selection` (`|GetArrayItem` (`self.SpawnedShapes`) (`self.CurrentIndex`)) false)
      (bind _result (`/Engine/EditorBlueprintResources/StandardMacros.DecrementInt` (`self.CurrentIndex`))
        (:`  `
          (`/Game/LabWork2/BP_Shape.Selection` (`|GetArrayItem` (`self.SpawnedShapes`) _result) true))))))

(event `Key|Three`
  (params (Key :type "Key Structure"))
  ; Move
  (:`Pressed`
    (set `self.bIsVertical` (not (`self.bIsVertical`)))))

(event `Key|One`
  (params (Key :type "Key Structure"))
  ; Move
  (:`Pressed`
    (if (`self.bIsVertical`)
      (`self.K2_AddActorWorldOffset` (`|GetArrayItem` (`self.SpawnedShapes`) (`self.CurrentIndex`)) (0.0 0.0 -50.0) false false)
      (else
        (`self.K2_AddActorWorldOffset` (`|GetArrayItem` (`self.SpawnedShapes`) (`self.CurrentIndex`)) (0.0 -50.0 0.0) false false)))))

(event `Key|Two`
  (params (Key :type "Key Structure"))
  ; Move
  (:`Pressed`
    (if (`self.bIsVertical`)
      (`self.K2_AddActorWorldOffset` (`|GetArrayItem` (`self.SpawnedShapes`) (`self.CurrentIndex`)) (0.0 0.0 50.0) false false)
      (else
        (`self.K2_AddActorWorldOffset` (`|GetArrayItem` (`self.SpawnedShapes`) (`self.CurrentIndex`)) (0.0 50.0 0.0) false false)))))

(fn `UserConstructionScript`)