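; BP_Book is an interactable book that deactivates a type of trap, selected by its TargetTrap value.
; The construction script picks the book mesh to match the trap type: spike, gas or axe.
; On Interact it passes the trap type to BP_BorisCharacter through CallOnTrapDeactivated and removes its box component.
; A timeline then animates the mesh's uniform scale before the actor destroys itself.
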(event `/Game/LabWork/Blueprints/Resources/BPI_Interactable.Interact`
  (bind _asbp_boris_character (cast `/Game/LabWork/Blueprints/BP_BorisCharacter` (`GameplayStatics.GetPlayerCharacter` 0)))
  (`/Game/LabWork/Blueprints/BP_BorisCharacter.OnTrapDeactivated` _asbp_boris_character (`self.TargetTrap`))
  (`ActorComponent.K2_DestroyComponent` (`self.Box`))
  (bind (_direction _newtrack_0) (`Timeline|Timeline`)
    (:`Update`
      (`SceneComponent.SetRelativeScale3D` (`self.StaticMesh`) (`KismetMathLibrary.MakeVector` _newtrack_0 _newtrack_0 _newtrack_0)))
    (:`Finished`
      (`self.K2_DestroyActor`))))

(fn `UserConstructionScript`
  (switch `/Game/LabWork/Blueprints/Resources/E_TrapType` (`self.TargetTrap`)
    (:`NewEnumerator1`
      (`StaticMeshComponent.SetStaticMesh` (`self.StaticMesh`) "/Game/Packets/Fantastic_Dungeon_Pack/meshes/props/small_deco/SM_PROP_book_dungeon_01.SM_PROP_book_dungeon_01"))
    (:`NewEnumerator2`
      (`StaticMeshComponent.SetStaticMesh` (`self.StaticMesh`) "/Game/Packets/Fantastic_Dungeon_Pack/meshes/props/small_deco/SM_PROP_book_dungeon_03.SM_PROP_book_dungeon_03"))
    (:`NewEnumerator3`
      (`StaticMeshComponent.SetStaticMesh` (`self.StaticMesh`) "/Game/Packets/Fantastic_Dungeon_Pack/meshes/props/small_deco/SM_PROP_book_dungeon_02.SM_PROP_book_dungeon_02"))))