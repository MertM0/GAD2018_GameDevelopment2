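; BP_MazeCell is a modular maze cell that builds its own room and spawns a trap and pickups.
; The Construction Script sizes and places floor, walls, roof and spotlight from CellSize, then hides disabled walls or roof by zeroing their scale.
; On BeginPlay it spawns the selected spike, gas or axe trap.
; If item spawning is allowed, chained random rolls spawn gold, a medkit or nothing.
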(event `self.ReceiveBeginPlay`
  (bind _returnvalue (`KismetMathLibrary.RandomIntegerInRange` 0 100))
  (bind _returnvalue_2 (`SceneComponent.K2_GetComponentLocation` (`self.TrapSpawnPoint`)))
  (bind _returnvalue_3 (`SceneComponent.K2_GetComponentLocation` (`self.ItemSpawnPoint`)))
  (`|ExecutionSequence`
    (:`then_0`
      ;[0 1 0 0.5] Trap Spawn
      (switch `/Game/LabWork/Blueprints/Resources/E_TrapType` (`self.TrapSelection`)
        (:`NewEnumerator1`
          (`|SpawnActorFromClass` "/Game/LabWork/Blueprints/BP_TrapSpike.BP_TrapSpike_C" (`KismetMathLibrary.MakeTransform` _returnvalue_2) "Undefined" "MultiplyWithRoot" null null))
        (:`NewEnumerator2`
          (`|SpawnActorFromClass` "/Game/LabWork/Blueprints/BP_TrapGas.BP_TrapGas_C" (`KismetMathLibrary.MakeTransform` _returnvalue_2) "Undefined" "MultiplyWithRoot" null null))
        (:`NewEnumerator3`
          (`|SpawnActorFromClass` "/Game/LabWork/Blueprints/BP_TrapAxe.BP_TrapAxe_C" (`KismetMathLibrary.MakeTransform` _returnvalue_2) "Undefined" "MultiplyWithRoot" null null))))
    (:`then_1`
      ;[1 0.63 0 0.5] Collectable Spawn
      (if (`self.CanSpawnItem`)
        (if (<= _returnvalue 30)
          (`|SpawnActorFromClass` "/Game/LabWork/Blueprints/BP_Gold.BP_Gold_C" (`KismetMathLibrary.MakeTransform` _returnvalue_3) "Undefined" "MultiplyWithRoot" null null)
          (elif (<= _returnvalue 50)
            (`|SpawnActorFromClass` "/Game/LabWork/Blueprints/BP_Medkit.BP_Medkit_C" (`KismetMathLibrary.MakeTransform` _returnvalue_3) "Undefined" "MultiplyWithRoot" null null)))))))

(fn `UserConstructionScript`
  (bind _cellsize (`self.CellSize`))
  (bind _spotlight (`self.SpotLight`))
  (bind _cellsize_2 (`self.CellSize`))
  (bind _cellsize_3 (`self.CellSize`))
  (bind _cellsize_4 (`self.CellSize`))
  (bind _cellsize_5 (`self.CellSize`))
  (bind _cellsize_6 (`self.CellSize`))
  (bind _returnvalue (* (`self.CellSize`) 100.0))
  (bind _returnvalue_2 (/ _returnvalue 2.0))
  (`|ExecutionSequence`
    (:`then_0`
      (`SceneComponent.SetRelativeScale3D` (`self.Floor`) (`KismetMathLibrary.MakeVector` _cellsize_2 _cellsize_2 (`self.WallThickness`)))
      (`SceneComponent.SetRelativeScale3D` (`self.WallWest`) (`KismetMathLibrary.MakeVector` _cellsize_5 (`self.WallThickness`) _cellsize_5))
      (`SceneComponent.K2_SetRelativeTransform` (`self.WallEast`) (`KismetMathLibrary.MakeTransform` (`KismetMathLibrary.MakeVector` 0.0 (* (`self.CellSize`) 90.0)) (struct) (`KismetMathLibrary.MakeVector` _cellsize (`self.WallThickness`) _cellsize)) false false)
      (`SceneComponent.K2_SetRelativeTransform` (`self.WallNorth`) (`KismetMathLibrary.MakeTransform` (`KismetMathLibrary.MakeVector` (* (`self.CellSize`) 10.0)) (struct :`Yaw` 90.0) (`KismetMathLibrary.MakeVector` _cellsize_3 (`self.WallThickness`) _cellsize_3)) false false)
      (`SceneComponent.K2_SetRelativeTransform` (`self.WallSouth`) (`KismetMathLibrary.MakeTransform` (`KismetMathLibrary.MakeVector` (* (`self.CellSize`) 100.0)) (struct :`Yaw` 90.0) (`KismetMathLibrary.MakeVector` _cellsize_6 (`self.WallThickness`) _cellsize_6)) false false)
      (`SceneComponent.K2_SetRelativeTransform` (`self.Roof`) (`KismetMathLibrary.MakeTransform` (`KismetMathLibrary.MakeVector` 0.0 0.0 (* (`self.CellSize`) 100.0)) (struct) (`KismetMathLibrary.MakeVector` _cellsize_4 _cellsize_4 (`self.WallThickness`))) false false)
      (`SceneComponent.K2_SetRelativeLocation` (`self.SpotLight`) (`KismetMathLibrary.MakeVector` _returnvalue_2 _returnvalue_2 _returnvalue) false false)
      (`LocalLightComponent.SetAttenuationRadius` _spotlight (* (`self.CellSize`) 110.0))
      (`LightComponent.SetIntensity` _spotlight (`self.LightIntensity`))
      (`LightComponent.SetLightColor` _spotlight (`self.LightColor`) true))
    (:`then_1`
      (`self.WallBool` (`self.EastBool`) (`self.WallEast`))
      (`self.WallBool` (`self.NorthBool`) (`self.WallNorth`))
      (`self.WallBool` (`self.SouthBool`) (`self.WallSouth`))
      (`self.WallBool` (`self.WestBool`) (`self.WallWest`))
      (`self.WallBool` (`self.RoofBool`) (`self.Roof`)))))

(fn `WallBool`
  (params (WallBool :type Boolean) (Wall :type "StaticMeshComponent Object Reference"))
  (if (not WallBool)
    (`SceneComponent.SetRelativeScale3D` Wall (0.0 0.0 0.0))))