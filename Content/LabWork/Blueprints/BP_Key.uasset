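; BP_Key is a colored key pickup that the player collects into the Boris character's key inventory.
; On BeginPlay, KeyColor selects a red or green material instance for both slots of the mesh.
; Interact adds the color to KeyInventory, prints a message and destroys the Box component, then a timeline drives the mesh's uniform scale before the actor destroys itself.
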(event `self.ReceiveBeginPlay`
  ; Set Key Color
  (switch `/Game/LabWork/Blueprints/Resources/E_KeyColors` (`self.KeyColor`)
    (:`NewEnumerator0`
      (`PrimitiveComponent.SetMaterial` (`self.StaticMesh`) 0 "/Engine/VREditor/LaserPointer/LaserPointerMaterialInst.LaserPointerMaterialInst")
      (`PrimitiveComponent.SetMaterial` (`self.StaticMesh`) 1 "/Engine/VREditor/LaserPointer/LaserPointerMaterialInst.LaserPointerMaterialInst"))
    (:`NewEnumerator1`
      (`PrimitiveComponent.SetMaterial` (`self.StaticMesh`) 0 "/Engine/VREditor/LaserPointer/LaserPointerMaterial_Inst.LaserPointerMaterial_Inst")
      (`PrimitiveComponent.SetMaterial` (`self.StaticMesh`) 1 "/Engine/VREditor/LaserPointer/LaserPointerMaterial_Inst.LaserPointerMaterial_Inst"))))

(event `/Game/LabWork/Blueprints/Resources/BPI_Interactable.Interact`
  (bind _keycolor (`self.KeyColor`))
  ; Interact
  (bind _asbp_boris_character (cast `/Game/LabWork/Blueprints/BP_BorisCharacter` (`GameplayStatics.GetPlayerCharacter` 0)))
  (`KismetArrayLibrary.Array_Add` (`/Game/LabWork/Blueprints/BP_BorisCharacter.KeyInventory` _asbp_boris_character) _keycolor)
  (`KismetSystemLibrary.PrintString` (`KismetStringLibrary.Concat_StrStr` "Key Acquired: " (`|GetEnumeratorNameAsString` _keycolor)) true true (struct :`R` 1.0 :`G` 0.802061 :`A` 1.0))
  (`ActorComponent.K2_DestroyComponent` (`self.Box`))
  (bind (_direction _newtrack_0) (`Timeline|Timeline`)
    (:`Update`
      (`SceneComponent.SetRelativeScale3D` (`self.StaticMesh`) (`KismetMathLibrary.MakeVector` _newtrack_0 _newtrack_0 _newtrack_0)))
    (:`Finished`
      (`self.K2_DestroyActor`))))

(fn `UserConstructionScript`)