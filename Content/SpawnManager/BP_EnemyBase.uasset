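; Base enemy actor that takes its health, damage and speed from an EnemyStats struct and drops loot when killed.
; On BeginPlay it copies those stats, writes type and health to a text label, and picks a Goblin, Skeleton, Orc or Mage skeletal mesh by enum.
; TakeDamage lowers health without refreshing the label; at zero it destroys the actor, then spawns BP_Loot with Gold scaled by Difficulty.
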(event `self.ReceiveBeginPlay`
  (bind _mesh (`self.Mesh`))
  (bind (_health _damage _speed) (break `/Game/SpawnManager/ST_EnemyStats` (`self.EnemyStats`)))
  (bind _output_get (set `self.CurrentHealth` _health))
  (set `self.AttackDamage` _damage)
  (set `self.MoveSpeed` _speed)
  (`TextRenderComponent.K2_SetText` (`self.TextRender`) (`KismetTextLibrary.Conv_StringToText` (`KismetStringLibrary.Concat_StrStr` (`|GetEnumeratorNameAsString` (`self.EEnemyType`)) "/" (`KismetStringLibrary.Conv_DoubleToString` _output_get))))
  (switch `/Game/SpawnManager/E_EnemyType` (`self.EEnemyType`)
    (:`NewEnumerator3`
      (`SkeletalMeshComponent.SetSkeletalMeshAsset` _mesh "/Game/SpawnManager/SKM_Goblin.SKM_Goblin"))
    (:`NewEnumerator0`
      (`SkeletalMeshComponent.SetSkeletalMeshAsset` _mesh "/Game/SpawnManager/SKM_Skeleton.SKM_Skeleton"))
    (:`NewEnumerator1`
      (`SkeletalMeshComponent.SetSkeletalMeshAsset` _mesh "/Game/SpawnManager/SKM_Orc.SKM_Orc"))
    (:`NewEnumerator2`
      (`SkeletalMeshComponent.SetSkeletalMeshAsset` _mesh "/Game/SpawnManager/SKM_Mage.SKM_Mage"))))

(fn `TakeDamage`
  (params (Damage :type "Float (double-precision)"))
  (returns (CurrentHealth :type "Float (double-precision)"))
  (bind _output_get (set `self.CurrentHealth` (- (`self.CurrentHealth`) Damage)))
  (if (<= _output_get 0.0)
    (`self.K2_DestroyActor`)
    (`|SpawnActorFromClass` "/Game/SpawnManager/BP_Loot.BP_Loot_C" (`self.GetTransform`) "Undefined" "MultiplyWithRoot" null (* (`self.Difficulty`) 100) null)
    (else
      (return _output_get))))

(fn `UserConstructionScript`)